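; Camera Blueprint that, when flagged as first-person, limits view pitch and creates the HUD with a context-sensitive crosshair.
; A self-retriggering event on a very short Delay line-traces forward from the camera on the Visibility channel.
; The hit actor's tag selects the cross, round or triangle crosshair through HUD booleans.
; A miss or untagged hit keeps the previous crosshair.
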(event `Check Switch Crosshair`
  (bind _cameracomponent (`self.CameraComponent`))
  (bind _hud_ref (`self.Hud Ref`))
  (bind _returnvalue (`SceneComponent.K2_GetComponentLocation` _cameracomponent))
  ;[1 0 0] Switch Crosshairs on HUD
  (bind (_outhit _returnvalue_2) (`KismetSystemLibrary.LineTraceSingle` _returnvalue (+ _returnvalue (* (`SceneComponent.GetForwardVector` _cameracomponent) 4000.0)) "TraceTypeQuery1"))
  (if _returnvalue_2
    (bind (_bblockinghit _binitialoverlap _time _distance _location _impactpoint _normal _impactnormal _physmat _hitactor) (`GameplayStatics.BreakHitResult` _outhit))
    (if (`self.ActorHasTag` _hitactor "Base_Crosshair")
      (set `/Game/UI/WBP_Hud.Cross?` true _hud_ref)
      (set `/Game/UI/WBP_Hud.Round?` false _hud_ref)
      (set `/Game/UI/WBP_Hud.Triangle?` false _hud_ref)
      (elif (`self.ActorHasTag` _hitactor "Secondary_Crosshair")
        (set `/Game/UI/WBP_Hud.Cross?` false _hud_ref)
        (set `/Game/UI/WBP_Hud.Round?` true _hud_ref)
        (set `/Game/UI/WBP_Hud.Triangle?` false _hud_ref)
        (elif (`self.ActorHasTag` _hitactor "Tertiary_Crosshair")
          (set `/Game/UI/WBP_Hud.Cross?` false _hud_ref)
          (set `/Game/UI/WBP_Hud.Round?` false _hud_ref)
          (set `/Game/UI/WBP_Hud.Triangle?` true _hud_ref)))))
  (`KismetSystemLibrary.Delay` 0.001)
  (`self.Check Switch Crosshair`))

(event `self.ReceiveBeginPlay`
  (bind _returnvalue (`GameplayStatics.GetPlayerCameraManager` 0))
  (if (`self.IsCamFPS?`)
    ;[0 0 0] Clamp Camera
    (set `PlayerCameraManager.ViewPitchMin` -60.0 _returnvalue)
    (set `PlayerCameraManager.ViewPitchMax` 32.0 _returnvalue)
    ;[1 0 0] Add HUD & Crosshair switch
    (bind _returnvalue_2 (`|CreateWidget` "/Game/UI/WBP_Hud.WBP_Hud_C" (`GameplayStatics.GetPlayerController` 0)))
    (bind _output_get (set `self.Hud Ref` _returnvalue_2))
    (`UserWidget.AddToViewport` _output_get 0)
    (`self.Check Switch Crosshair`)))

(fn `UserConstructionScript`)